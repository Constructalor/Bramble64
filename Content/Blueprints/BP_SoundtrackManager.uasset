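; BP_SoundtrackManager is an actor that drives the music's CutoffFreq parameter from player movement and handles an escape music switch.
; Each tick it derives a cutoff from the player pawn's horizontal speed, far higher and more speed-sensitive while BP_ThirdPersonCharacter is ramming.
; The value is smoothed with FInterpTo before reaching the Audio component.
; EscapeTransition calls a short fade-out, then immediately sets and plays the W_BrambleLap1_FeelingSHOCKED track.
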(event Custom|EscapeTransition
  (bind _audio (Variables|Default|GetAudio))
  (Audio|Components|Audio|FadeOut _audio 0.2 0.0 "Linear" :!class /Script/Engine.AudioComponent)
  (Audio|Components|Audio|SetSound _audio "/Game/Audio/Music/W_BrambleLap1_FeelingSHOCKED.W_BrambleLap1_FeelingSHOCKED")
  (Audio|Components|Audio|Play _audio 0.0))

(event EventBeginPlay)

(event Collision|EventActorBeginOverlap
  (params (OtherActor :type Actor%20Object%20Reference)))

(event EventTick
  (params (DeltaSeconds :type Float%20%28single-precision%29))
  (bind _returnvalue (Game|Player|GetPlayerPawn 0))
  (bind _returnvalue_2 (Transformation|GetVelocity _returnvalue))
  (bind (_x _y) (Math|Vector|BreakVector _returnvalue_2))
  (bind _returnvalue_3 (Math|Vector|MakeVector _x _y 0.0))
  (bind _returnvalue_4 (Math|Vector|VectorLength _returnvalue_3))
  (bind _asbp_third_person_character (Utilities|Casting|CastToBP_ThirdPersonCharacter _returnvalue))
  (bind _output_get (Variables|Default|SetCutoffFreq (Math|Interpolation|FInterpTo (Variables|Default|GetCutoffFreq) (select (Variables|/Game/ThirdPerson/Blueprints/BP_ThirdPersonCharacter.BP_ThirdPersonCharacter_C|GetIsRamming _asbp_third_person_character) (+ (* _returnvalue_4 0.5) 1e+03) (+ (* _returnvalue_4 0.03) 2e+01)) (Utilities|Time|GetWorldDeltaSeconds) 5.0)))
  (Audio|Parameter|SetFloatParameter (Variables|Default|GetAudio) "CutoffFreq" _output_get :!class /Script/Engine.AudioComponent))

(fn ConstructionScript)