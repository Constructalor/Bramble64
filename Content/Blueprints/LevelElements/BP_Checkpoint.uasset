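; BP_Checkpoint is a checkpoint level element that switches its glow and audio on and off through Activate and Deactivate events.
; The construction script gives the Cube a dynamic effect material and passes it the actor's location as a vector parameter.
; A timeline, played forward or reversed, blends the material's emissive and speed parameters.
; Both events play the activation sound, while the ambience sound starts on activation and stops on deactivation.
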(event Custom|Deactivate
  (bind _dynamicfxmat (Variables|Default|GetDynamicFXMat))
  (Audio|Components|Audio|Stop (Variables|Default|GetAmbience))
  (Audio|Components|Audio|Play (Variables|Default|GetActivation) 0.0)
  (bind _alpha (Timeline|MaterialFXTimeline Reverse)
    (:Update
      (Rendering|Material|SetScalarParameterValue _dynamicfxmat "EmissiveMultiplier" (Math|Float|Lerp 0.75 1.1 _alpha) :!class /Script/Engine.MaterialInstanceDynamic)
      (Rendering|Material|SetScalarParameterValue _dynamicfxmat "EmissivePower" (Math|Float|Lerp 5.0 25.0 _alpha) :!class /Script/Engine.MaterialInstanceDynamic)
      (Rendering|Material|SetScalarParameterValue _dynamicfxmat "Speed" (Math|Float|Lerp 1e-05 6e-05 _alpha) :!class /Script/Engine.MaterialInstanceDynamic))
    (:Finished
      (Audio|Components|Audio|FadeOut (Variables|Default|GetActivation) 0.1 0.0 "Linear" :!class /Script/Engine.AudioComponent))))

(event Custom|Activate
  (bind _dynamicfxmat (Variables|Default|GetDynamicFXMat))
  (Audio|Components|Audio|Play (Variables|Default|GetActivation) 0.0)
  (bind _alpha (Timeline|MaterialFXTimeline Play)
    (:Update
      (Rendering|Material|SetScalarParameterValue _dynamicfxmat "EmissiveMultiplier" (Math|Float|Lerp 0.75 1.1 _alpha) :!class /Script/Engine.MaterialInstanceDynamic)
      (Rendering|Material|SetScalarParameterValue _dynamicfxmat "EmissivePower" (Math|Float|Lerp 5.0 25.0 _alpha) :!class /Script/Engine.MaterialInstanceDynamic)
      (Rendering|Material|SetScalarParameterValue _dynamicfxmat "Speed" (Math|Float|Lerp 1e-05 6e-05 _alpha) :!class /Script/Engine.MaterialInstanceDynamic))
    (:Finished
      (Audio|Components|Audio|FadeOut (Variables|Default|GetActivation) 0.1 0.0 "Linear" :!class /Script/Engine.AudioComponent))))

(event EventBeginPlay)

(event Collision|EventActorBeginOverlap
  (params (OtherActor :type Actor%20Object%20Reference)))

(event EventTick
  (params (DeltaSeconds :type Float%20%28single-precision%29)))

(fn ConstructionScript
  (bind _returnvalue (Transformation|GetActorLocation))
  (bind _returnvalue_2 (Rendering|Material|CreateDynamicMaterialInstance "/Game/VFX/Teleporter/MI_Checkpoint_Effect.MI_Checkpoint_Effect" "None" "None" :!class /Script/Engine.KismetMaterialLibrary))
  (bind _output_get (Variables|Default|SetDynamicFXMat _returnvalue_2))
  (Rendering|Material|SetMaterial (Variables|Default|GetCube) 1 _output_get)
  (Rendering|Material|SetVectorParameterValue _output_get "Location" (Math|Color|MakeColor (.x _returnvalue) (.y _returnvalue) (.z _returnvalue)) :!class /Script/Engine.MaterialInstanceDynamic))