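; BP_Enemy is an enemy actor that explodes when killed, then either destroys itself or respawns after a delay, depending on DeathType.
; KillEnemy plays the explosion sound and Niagara effect, with Disable and Enable toggling collision and visibility for respawning.
; Enable leaves the Widget hidden.
; The HitSphere overlap event is empty, and the character attack/dive speed checks that would call KillEnemy are disconnected.
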(event OnComponentBeginOverlap(HitSphere)
  (params (OverlappedComponent :type Primitive%20Component%20Object%20Reference) (OtherActor :type Actor%20Object%20Reference) (OtherComp :type Primitive%20Component%20Object%20Reference) (OtherBodyIndex :type Integer) (bFromSweep :type Boolean) (SweepResult :type Hit%20Result%20Structure%20%28by%20ref%29)))

(event Custom|KillEnemy
  (Audio|PlaySoundatLocation "/Game/Audio/SFX/W_Explosion.W_Explosion" (Transformation|GetActorLocation) "0, 0, 0" 2.0 1.0 0.0 "/Game/Audio/SFX/SA_Default.SA_Default" 0 0 0)
  (Niagara|SpawnSystematLocation "/Game/VFX/Explosion/NS_Explosion.NS_Explosion" (Transformation|GetActorLocation))
  (switch Utilities|FlowControl|Switch|SwitchonE_DeathType (Variables|Default|GetDeathType)
    (:NewEnumerator0
      (Actor|DestroyActor))
    (:NewEnumerator1
      (CallFunction|Disable)
      (Utilities|FlowControl|Delay (Variables|Default|GetTimeToRespawn))
      (CallFunction|Enable))))

(event Custom|Enable
  (bind _sphere (Variables|Default|GetSphere))
  (Collision|SetCollisionEnabled (Variables|Default|GetHitSphere) "QueryOnly")
  (Rendering|SetVisibility _sphere true false)
  (Collision|SetCollisionEnabled _sphere "QueryAndPhysics")
  (Variables|Default|SetEnabled true))

(event Custom|Disable
  (bind _sphere (Variables|Default|GetSphere))
  (Collision|SetCollisionEnabled (Variables|Default|GetHitSphere) "NoCollision")
  (Rendering|SetVisibility _sphere false false)
  (Collision|SetCollisionEnabled _sphere "NoCollision")
  (Rendering|SetVisibility (Variables|Default|GetWidget) false false)
  (Variables|Default|SetEnabled false))

(fn ConstructionScript)